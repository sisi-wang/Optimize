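; BP_Land_ is a three-lane track segment for a parkour runner, built from left, center and right BP_land_piece child actors.
; On BeginPlay it shuffles slot and piece arrays to place up to two barriers, leaving a lane free, and randomly adds tools to unblocked pieces.
; When the parkour character enters its box, it calls LoopTrack on the game mode through a DoOnce that resets shortly after exit.
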(event `self.ReceiveBeginPlay`
  (bind _piece_array (`self.piece array`))
  (bind _asbp_land_piece (cast `/Game/parkour/Blueprint/BP_land_piece` (`ChildActorComponent.ChildActor` (`self.BP_land_piece_right`))))
  (set `self.rightland` _asbp_land_piece)
  (bind _asbp_land_piece_2 (cast `/Game/parkour/Blueprint/BP_land_piece` (`ChildActorComponent.ChildActor` (`self.BP_land_piece_left`))))
  (set `self.leftland` _asbp_land_piece_2)
  (bind _asbp_land_piece_3 (cast `/Game/parkour/Blueprint/BP_land_piece` (`ChildActorComponent.ChildActor` (`self.BP_land_piece_center`))))
  (set `self.centerland` _asbp_land_piece_3)
  (`KismetArrayLibrary.Array_Add` _piece_array (`self.rightland`))
  (`KismetArrayLibrary.Array_Add` _piece_array (`self.leftland`))
  (`KismetArrayLibrary.Array_Add` _piece_array (`self.centerland`))
  (`self.Add barriers`))

(event `self.Box.OnComponentBeginOverlap`
  (params (OverlappedComponent :type "PrimitiveComponent Object Reference") (OtherActor :type "Actor Object Reference") (OtherComp :type "PrimitiveComponent Object Reference") (OtherBodyIndex :type Integer) (bFromSweep :type Boolean) (SweepResult :type "HitResult Structure (by ref)"))
  (cast `/Game/parkour/Blueprint/BP_parkourchr` OtherActor)
  (`/Engine/EditorBlueprintResources/StandardMacros.DoOnce` false :!label _label
    (:`Completed`
      (bind _asbp_gamemode (cast `/Game/parkour/gamemode/BP_gamemode` (`GameplayStatics.GetGameMode`)))
      (`/Game/parkour/gamemode/BP_gamemode.LoopTrack` _asbp_gamemode self))))

(event `self.Box.OnComponentEndOverlap`
  (params (OverlappedComponent :type "PrimitiveComponent Object Reference") (OtherActor :type "Actor Object Reference") (OtherComp :type "PrimitiveComponent Object Reference") (OtherBodyIndex :type Integer))
  (cast `/Game/parkour/Blueprint/BP_parkourchr` OtherActor)
  (`KismetSystemLibrary.Delay` 1.0)
  (goto _label :!via `Reset`))

(fn `Add barriers`
  (locals (NewLocalVar :type "/Game/parkour/Blueprint/BP_land_piece Object Reference") (`piece slot local` :type "Array of Float (double-precision)"))
  (bind _piece_array (`self.piece array`))
  (bind _result (`BlueprintSetLibrary.Set_ToArray` (`self.piece slot`)))
  (bind _output_get (set `local.piece slot local` _result))
  (`KismetArrayLibrary.Array_Shuffle` _output_get)
  ; 0no barriers1 1barrier 2 2barriers
  (switch `int` (`KismetMathLibrary.FTrunc` (`|GetArrayItem` (`local.piece slot local`)))
    (:`0`
      (`KismetArrayLibrary.Array_Shuffle` (`local.piece slot local`))
      ; spawn tool/coin 0-11-2 2-3
      (switch `int` (`KismetMathLibrary.FTrunc` (`|GetArrayItem` (`local.piece slot local`)))
        (:`0`
          (`self.one tool switch piece`))
        (:`1`
          (`self.two tool switch piece`))
        (:`2`
          (`self.three tool seitch piece`))))
    (:`1`
      (`KismetArrayLibrary.Array_Shuffle` (`self.piece array`))
      (`/Game/parkour/Blueprint/BP_land_piece.Add Barrier` (`|GetArrayItem` (`self.piece array`)))
      (switch `int` (`KismetMathLibrary.RandomIntegerInRange` 0 2)
        (:`1`
          (switch `int` (`KismetMathLibrary.RandomIntegerInRange` 0 1)
            (:`0`
              (`/Game/parkour/Blueprint/BP_land_piece.Add Tool` (`|GetArrayItem` (`self.piece array`) 1)))
            (:`1`
              (`/Game/parkour/Blueprint/BP_land_piece.Add Tool` (`|GetArrayItem` (`self.piece array`) 1)))))
        (:`2`
          (`/Game/parkour/Blueprint/BP_land_piece.Add Tool` (`|GetArrayItem` (`self.piece array`) 1))
          (`/Game/parkour/Blueprint/BP_land_piece.Add Tool` (`|GetArrayItem` (`self.piece array`) 2)))))
    (:`2`
      (`KismetArrayLibrary.Array_Shuffle` (`self.piece array`))
      (`/Game/parkour/Blueprint/BP_land_piece.Add Barrier` (`|GetArrayItem` _piece_array))
      (`/Game/parkour/Blueprint/BP_land_piece.Add Barrier` (`|GetArrayItem` _piece_array 1))
      ; 0 donot spawn tool 1 spawn tool
      (switch `int` (`KismetMathLibrary.RandomIntegerInRange` 0 1)
        (:`1`
          (`/Game/parkour/Blueprint/BP_land_piece.Add Tool` (`|GetArrayItem` (`self.piece array`) 2)))))))

(fn `UserConstructionScript`)