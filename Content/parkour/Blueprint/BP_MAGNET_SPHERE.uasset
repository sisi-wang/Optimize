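; BP_MAGNET_SPHERE is a temporary coin magnet power-up for the parkour game that destroys itself ten seconds after spawning.
; Each tick it teleports to the first player pawn's location, so it follows the player.
; When a BP_Coin begins overlapping its Sphere, it calls MagnetActive on that coin.
; Debug prints of the position and magnet hits remain in the graph.
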(event `self.ReceiveBeginPlay`
  (`KismetSystemLibrary.Delay` 10.0)
  (`self.K2_DestroyActor`))

(event `self.ReceiveTick`
  (params (DeltaSeconds :type "Float (single-precision)"))
  (bind _returnvalue (`self.K2_GetActorLocation` (`GameplayStatics.GetPlayerPawn` 0)))
  (`|ExecutionSequence`
    (:`then_0`
      (`self.K2_SetActorLocation` _returnvalue)
      (`KismetSystemLibrary.PrintString` (`KismetStringLibrary.Conv_VectorToString` _returnvalue)))))

(event `self.Sphere.OnComponentBeginOverlap`
  (params (OverlappedComponent :type "PrimitiveComponent Object Reference") (OtherActor :type "Actor Object Reference") (OtherComp :type "PrimitiveComponent Object Reference") (OtherBodyIndex :type Integer) (bFromSweep :type Boolean) (SweepResult :type "HitResult Structure (by ref)"))
  (bind _asbp_coin (cast `/Game/parkour/Blueprint/BP_Coin` OtherActor))
  (`KismetSystemLibrary.PrintString` "MAGNET")
  (`/Game/parkour/Blueprint/BP_Coin.MagnetActive?` _asbp_coin))

(fn `UserConstructionScript`)