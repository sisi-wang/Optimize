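; BP_ObstacleBase is a parkour obstacle base Blueprint that provides helper functions to switch an obstacle on and off.
; EnableCollision shows a given static mesh with blocking physics-only collision and makes its companion box a query-only overlap volume.
; UnableCollision hides the mesh and disables collision on both components, ignoring all channels.
; The event graph and construction script contain no logic.
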(fn `Enable Collision`
  (params (StaticMesh :type "StaticMeshComponent Object Reference") (componentbox :type "BoxComponent Object Reference"))
  (`SceneComponent.SetVisibility` StaticMesh true false)
  (`PrimitiveComponent.SetCollisionEnabled` StaticMesh "PhysicsOnly")
  (`PrimitiveComponent.SetCollisionResponseToAllChannels` StaticMesh "ECR_Block")
  (`PrimitiveComponent.SetCollisionEnabled` componentbox "QueryOnly")
  (`PrimitiveComponent.SetCollisionResponseToAllChannels` componentbox "ECR_Overlap"))

(fn `Unable Collision`
  (params (StaticMesh :type "StaticMeshComponent Object Reference") (`Component box` :type "BoxComponent Object Reference"))
  (`SceneComponent.SetVisibility` StaticMesh false false)
  (`PrimitiveComponent.SetCollisionEnabled` StaticMesh "NoCollision")
  (`PrimitiveComponent.SetCollisionResponseToAllChannels` StaticMesh "ECR_Ignore")
  (`PrimitiveComponent.SetCollisionEnabled` `Component box` "NoCollision")
  (`PrimitiveComponent.SetCollisionResponseToAllChannels` `Component box` "ECR_Ignore"))

(fn `UserConstructionScript`)