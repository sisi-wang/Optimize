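; Heart pickup for the parkour game that grants the player character temporary protection.
; It gains a rotating movement component on BeginPlay; a Box overlap sets PROTECT on BP_parkourchr and clears it after a five-second delay.
; A DoOnce, reset on end overlap, guards the trigger.
; Pickup hides the actor and disables collision rather than destroying it; Enablecollection reverses this but is not called in this graph.
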(event `self.ReceiveBeginPlay`
  (`AddComponent|NODE_AddRotatingMovementComponent-0`))

(event `self.Box.OnComponentBeginOverlap`
  (params (OverlappedComponent :type "PrimitiveComponent Object Reference") (OtherActor :type "Actor Object Reference") (OtherComp :type "PrimitiveComponent Object Reference") (OtherBodyIndex :type Integer) (bFromSweep :type Boolean) (SweepResult :type "HitResult Structure (by ref)"))
  (bind _asbp_parkourchr (cast `/Game/parkour/Blueprint/BP_parkourchr` OtherActor))
  (`/Engine/EditorBlueprintResources/StandardMacros.DoOnce` false :!label _label
    (:`Completed`
      (set `/Game/parkour/Blueprint/BP_parkourchr.PROTECT?` true _asbp_parkourchr)
      (`|ExecutionSequence`
        (:`then_0`
          (`self.unable collection`))
        (:`then_1`
          (`KismetSystemLibrary.Delay` 5.0)
          (set `/Game/parkour/Blueprint/BP_parkourchr.PROTECT?` false _asbp_parkourchr))))))

(event `self.Box.OnComponentEndOverlap`
  (params (OverlappedComponent :type "PrimitiveComponent Object Reference") (OtherActor :type "Actor Object Reference") (OtherComp :type "PrimitiveComponent Object Reference") (OtherBodyIndex :type Integer))
  (cast `/Game/parkour/Blueprint/BP_parkourchr` OtherActor)
  (goto _label :!via `Reset`))

(fn `enablecollection`
  (`self.SetActorHiddenInGame` false)
  (`PrimitiveComponent.SetCollisionEnabled` (`self.Box`) "QueryOnly")
  (`PrimitiveComponent.SetCollisionEnabled` (`self.SM_Heart`) "QueryOnly"))

(fn `unable collection`
  (`self.SetActorHiddenInGame` true)
  (`PrimitiveComponent.SetCollisionEnabled` (`self.SM_Heart`) "NoCollision")
  (`PrimitiveComponent.SetCollisionEnabled` (`self.Box`) "NoCollision"))

(fn `UserConstructionScript`)