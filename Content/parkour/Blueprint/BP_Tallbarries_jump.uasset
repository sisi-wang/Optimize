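; Tall barrier obstacle for the parkour game that auto-launches the player over it and penalizes contact.
; Box_0 overlap launches a grounded BP_parkourchr upward and along X, scaling height with walk speed; a DoOnce resets on exit.
; Box1 overlap hides the obstacle and disables collision if the character is protected, otherwise calls the character's Over after a short delay.
; EnableCollision restores visibility and collision, but is not called within this Blueprint.
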(event `self.Box_0.OnComponentBeginOverlap`
  (params (OverlappedComponent :type "PrimitiveComponent Object Reference") (OtherActor :type "Actor Object Reference") (OtherComp :type "PrimitiveComponent Object Reference") (OtherBodyIndex :type Integer) (bFromSweep :type Boolean) (SweepResult :type "HitResult Structure (by ref)"))
  (bind _asbp_parkourchr (cast `/Game/parkour/Blueprint/BP_parkourchr` OtherActor))
  (`/Engine/EditorBlueprintResources/StandardMacros.DoOnce` false :!label _label
    (:`Completed`
      (bind _charactermovement (`Character.CharacterMovement` _asbp_parkourchr))
      (if (not (`NavMovementInterface.IsFalling` _charactermovement))
        (`Character.LaunchCharacter` _asbp_parkourchr (`KismetMathLibrary.MakeVector` 100.0 0.0 (+ (`self.jump`) (* (`CharacterMovementComponent.MaxWalkSpeed` _charactermovement) 0.5))) false true)))))

(event `self.Box_0.OnComponentEndOverlap`
  (params (OverlappedComponent :type "PrimitiveComponent Object Reference") (OtherActor :type "Actor Object Reference") (OtherComp :type "PrimitiveComponent Object Reference") (OtherBodyIndex :type Integer))
  (cast `/Game/parkour/Blueprint/BP_parkourchr` OtherActor)
  (goto _label :!via `Reset`))

(event `self.Box1.OnComponentBeginOverlap`
  (params (OverlappedComponent :type "PrimitiveComponent Object Reference") (OtherActor :type "Actor Object Reference") (OtherComp :type "PrimitiveComponent Object Reference") (OtherBodyIndex :type Integer) (bFromSweep :type Boolean) (SweepResult :type "HitResult Structure (by ref)"))
  (bind _asbp_parkourchr (cast `/Game/parkour/Blueprint/BP_parkourchr` OtherActor))
  (if (`/Game/parkour/Blueprint/BP_parkourchr.PROTECT?` _asbp_parkourchr)
    (`self.unable collision`)
    (else
      (`KismetSystemLibrary.Delay` 0.2)
      (`/Game/parkour/Blueprint/BP_parkourchr.over` _asbp_parkourchr))))

(fn `enable collision`
  (`self.SetActorHiddenInGame` false)
  (`PrimitiveComponent.SetCollisionEnabled` (`self.Box_0`) "QueryOnly")
  (`PrimitiveComponent.SetCollisionEnabled` (`self.Box1`) "QueryOnly")
  (`PrimitiveComponent.SetCollisionEnabled` (`self.Cube`) "QueryOnly")
  (`PrimitiveComponent.SetCollisionEnabled` (`self.barrier`) "QueryAndPhysics"))

(fn `unable collision`
  (`self.SetActorHiddenInGame` true)
  (`PrimitiveComponent.SetCollisionEnabled` (`self.barrier`) "NoCollision")
  (`PrimitiveComponent.SetCollisionEnabled` (`self.Box1`) "NoCollision")
  (`PrimitiveComponent.SetCollisionEnabled` (`self.Cube`) "NoCollision")
  (`PrimitiveComponent.SetCollisionEnabled` (`self.Box_0`) "NoCollision"))

(fn `UserConstructionScript`)