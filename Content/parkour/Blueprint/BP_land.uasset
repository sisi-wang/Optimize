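; BP_land is a ground segment for a three-lane parkour runner that places obstacles and pickups and drives track extension.
; Its Box overlap increments the parkour character's ThroughLand counter, and on reaching three resets it and asks BP_gamemode to AddLand for the next three indices.
; AddBarrier spawns one or two barriers on even indices, or one to three props on odd ones, at random Left, Center and Right points.
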(event `self.ReceiveBeginPlay`
  (bind _asbp_gamemode (cast `/Game/parkour/gamemode/BP_gamemode` (`GameplayStatics.GetGameMode`)))
  (set `self.As BP Gamemode` _asbp_gamemode))

(event `self.Box.OnComponentBeginOverlap`
  (params (OverlappedComponent :type "PrimitiveComponent Object Reference") (OtherActor :type "Actor Object Reference") (OtherComp :type "PrimitiveComponent Object Reference") (OtherBodyIndex :type Integer) (bFromSweep :type Boolean) (SweepResult :type "HitResult Structure (by ref)"))
  (bind _asbp_parkourchr (cast `/Game/parkour/Blueprint/BP_parkourchr` OtherActor))
  (bind _output_get (set `self.As BP Parkourchr` _asbp_parkourchr))
  (bind _output_get_2 (set `/Game/parkour/Blueprint/BP_parkourchr.through land` (+ (`/Game/parkour/Blueprint/BP_parkourchr.through land` _output_get) 1) _output_get))
  (if (>= _output_get_2 3)
    (set `/Game/parkour/Blueprint/BP_parkourchr.through land` 0 _output_get)
    (bind _asbp_gamemode (cast `/Game/parkour/gamemode/BP_gamemode` (`GameplayStatics.GetGameMode`)))
    (bind _landend (`/Game/parkour/gamemode/BP_gamemode.Landend` _asbp_gamemode))
    (`/Game/parkour/gamemode/BP_gamemode.add land` _asbp_gamemode _landend (+ _landend 3))))

(fn `Add Barrier`
  (params (INDEX :type Integer))
  ; 这块生成不生成障碍
  (if (== (mod INDEX 2) 0)
    ; 生成几个障碍
    (switch `int` (`KismetMathLibrary.RandomIntegerInRange` 0 2)
      (:`0`
        ; 在哪个轨道生成障碍
        (switch `int` (`KismetMathLibrary.RandomIntegerInRange` 0 2) :!label _label
          (:`0`
            (`|SpawnActorFromClass` (`self.barrier num`) (`KismetMathLibrary.MakeTransform` (`SceneComponent.K2_GetComponentLocation` (`self.left_point`))) "Undefined" "MultiplyWithRoot" null null))
          (:`1`
            (`|SpawnActorFromClass` (`self.barrier num`) (`KismetMathLibrary.MakeTransform` (`SceneComponent.K2_GetComponentLocation` (`self.center_point`))) "Undefined" "MultiplyWithRoot" null null))
          (:`2`
            (`|SpawnActorFromClass` (`self.barrier num`) (`KismetMathLibrary.MakeTransform` (`SceneComponent.K2_GetComponentLocation` (`self.right_point`))) "Undefined" "MultiplyWithRoot" null null))))
      (:`1`
        (goto _label))
      (:`2`
        (switch `int` (`KismetMathLibrary.RandomIntegerInRange` 0 2)
          (:`0`
            (`|SpawnActorFromClass` (`self.barrier num`) (`KismetMathLibrary.MakeTransform` (`SceneComponent.K2_GetComponentLocation` (`self.left_point`))) "Undefined" "MultiplyWithRoot" null null)
            (`|SpawnActorFromClass` (`self.barrier num`) (`KismetMathLibrary.MakeTransform` (`SceneComponent.K2_GetComponentLocation` (`self.center_point`))) "Undefined" "MultiplyWithRoot" null null))
          (:`1`
            (`|SpawnActorFromClass` (`self.barrier num`) (`KismetMathLibrary.MakeTransform` (`SceneComponent.K2_GetComponentLocation` (`self.center_point`))) "Undefined" "MultiplyWithRoot" null null)
            (`|SpawnActorFromClass` (`self.barrier num`) (`KismetMathLibrary.MakeTransform` (`SceneComponent.K2_GetComponentLocation` (`self.right_point`))) "Undefined" "MultiplyWithRoot" null null))
          (:`2`
            (`|SpawnActorFromClass` (`self.barrier num`) (`KismetMathLibrary.MakeTransform` (`SceneComponent.K2_GetComponentLocation` (`self.left_point`))) "Undefined" "MultiplyWithRoot" null null)
            (`|SpawnActorFromClass` (`self.barrier num`) (`KismetMathLibrary.MakeTransform` (`SceneComponent.K2_GetComponentLocation` (`self.right_point`))) "Undefined" "MultiplyWithRoot" null null)))))
    (else
      (switch `int` (`KismetMathLibrary.RandomIntegerInRange` 0 3)
        (:`0`
          ; 在哪个轨道生成
          (switch `int` (`KismetMathLibrary.RandomIntegerInRange` 0 2) :!label _label_2
            (:`0`
              (`|SpawnActorFromClass` (`self.prop num`) (`KismetMathLibrary.MakeTransform` (`SceneComponent.K2_GetComponentLocation` (`self.left_point`))) "Undefined" "MultiplyWithRoot" null null))
            (:`1`
              (`|SpawnActorFromClass` (`self.prop num`) (`KismetMathLibrary.MakeTransform` (`SceneComponent.K2_GetComponentLocation` (`self.center_point`))) "Undefined" "MultiplyWithRoot" null null))
            (:`2`
              (`|SpawnActorFromClass` (`self.prop num`) (`KismetMathLibrary.MakeTransform` (`SceneComponent.K2_GetComponentLocation` (`self.right_point`))) "Undefined" "MultiplyWithRoot" null null))))
        (:`1`
          (goto _label_2))
        (:`2`
          (switch `int` (`KismetMathLibrary.RandomIntegerInRange` 0 2)
            (:`0`
              (`|SpawnActorFromClass` (`self.prop num`) (`KismetMathLibrary.MakeTransform` (`SceneComponent.K2_GetComponentLocation` (`self.left_point`))) "Undefined" "MultiplyWithRoot" null null)
              (`|SpawnActorFromClass` (`self.prop num`) (`KismetMathLibrary.MakeTransform` (`SceneComponent.K2_GetComponentLocation` (`self.center_point`))) "Undefined" "MultiplyWithRoot" null null))
            (:`1`
              (`|SpawnActorFromClass` (`self.prop num`) (`KismetMathLibrary.MakeTransform` (`SceneComponent.K2_GetComponentLocation` (`self.center_point`))) "Undefined" "MultiplyWithRoot" null null)
              (`|SpawnActorFromClass` (`self.prop num`) (`KismetMathLibrary.MakeTransform` (`SceneComponent.K2_GetComponentLocation` (`self.right_point`))) "Undefined" "MultiplyWithRoot" null null))
            (:`2`
              (`|SpawnActorFromClass` (`self.prop num`) (`KismetMathLibrary.MakeTransform` (`SceneComponent.K2_GetComponentLocation` (`self.left_point`))) "Undefined" "MultiplyWithRoot" null null)
              (`|SpawnActorFromClass` (`self.prop num`) (`KismetMathLibrary.MakeTransform` (`SceneComponent.K2_GetComponentLocation` (`self.right_point`))) "Undefined" "MultiplyWithRoot" null null))))
        (:`3`
          (switch `int` (`KismetMathLibrary.RandomIntegerInRange` 0 2)
            (:`0`
              (`|SpawnActorFromClass` (`self.prop num`) (`KismetMathLibrary.MakeTransform` (`SceneComponent.K2_GetComponentLocation` (`self.left_point`))) "Undefined" "MultiplyWithRoot" null null)
              (`|SpawnActorFromClass` (`self.prop num`) (`KismetMathLibrary.MakeTransform` (`SceneComponent.K2_GetComponentLocation` (`self.center_point`))) "Undefined" "MultiplyWithRoot" null null)
              (`|SpawnActorFromClass` (`self.prop num`) (`KismetMathLibrary.MakeTransform` (`SceneComponent.K2_GetComponentLocation` (`self.right_point`))) "Undefined" "MultiplyWithRoot" null null))
            (:`1`
              (`|SpawnActorFromClass` (`self.prop num`) (`KismetMathLibrary.MakeTransform` (`SceneComponent.K2_GetComponentLocation` (`self.center_point`))) "Undefined" "MultiplyWithRoot" null null)
              (`|SpawnActorFromClass` (`self.prop num`) (`KismetMathLibrary.MakeTransform` (`SceneComponent.K2_GetComponentLocation` (`self.right_point`))) "Undefined" "MultiplyWithRoot" null null)
              (`|SpawnActorFromClass` (`self.prop num`) (`KismetMathLibrary.MakeTransform` (`SceneComponent.K2_GetComponentLocation` (`self.left_point`))) "Undefined" "MultiplyWithRoot" null null))
            (:`2`
              (`|SpawnActorFromClass` (`self.prop num`) (`KismetMathLibrary.MakeTransform` (`SceneComponent.K2_GetComponentLocation` (`self.left_point`))) "Undefined" "MultiplyWithRoot" null null)
              (`|SpawnActorFromClass` (`self.prop num`) (`KismetMathLibrary.MakeTransform` (`SceneComponent.K2_GetComponentLocation` (`self.right_point`))) "Undefined" "MultiplyWithRoot" null null)
              (`|SpawnActorFromClass` (`self.prop num`) (`KismetMathLibrary.MakeTransform` (`SceneComponent.K2_GetComponentLocation` (`self.center_point`))) "Undefined" "MultiplyWithRoot" null null))))))))

(fn `UserConstructionScript`)