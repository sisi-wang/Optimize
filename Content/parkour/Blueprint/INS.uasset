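; INS is a parkour game Blueprint that saves and loads player score records through a BP_Savegame slot.
; SavePlayerScore loads the existing save or creates a new one, appends a name and score entry to its Playerdata array, then writes it back to the slot.
; LoadSaveData returns that Playerdata array when the slot exists, or nothing otherwise.
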(fn `LoadSaveData`
  (returns (playerdata :type "Array of /Game/parkour/Blueprint/S_Playerdata Structure"))
  (bind _returnvalue (`GameplayStatics.DoesSaveGameExist` (`self.slotName`)))
  (if _returnvalue
    (bind _returnvalue_2 (`GameplayStatics.LoadGameFromSlot` (`self.slotName`)))
    (bind _asbp_savegame (cast `/Game/parkour/Blueprint/BP_Savegame` _returnvalue_2))
    (return (`/Game/parkour/Blueprint/BP_Savegame.playerdata` _asbp_savegame))
    (else
      (return))))

(fn `SavePlayerScore`
  (params (playerName :type String) (score :type Integer))
  (bind _returnvalue (`GameplayStatics.DoesSaveGameExist` (`self.slotName`)))
  (if _returnvalue
    (bind _returnvalue_2 (`GameplayStatics.LoadGameFromSlot` (`self.slotName`)))
    (bind _asbp_savegame (cast `/Game/parkour/Blueprint/BP_Savegame` _returnvalue_2))
    (set `self.recordData` _asbp_savegame)
    (else
      (bind _returnvalue_3 (`GameplayStatics.CreateSaveGameObject` "/Game/parkour/Blueprint/BP_Savegame.BP_Savegame_C"))
      (set `self.recordData` _returnvalue_3)))
  (`KismetArrayLibrary.Array_Add` (`/Game/parkour/Blueprint/BP_Savegame.playerdata` (`self.recordData`)) (make `/Game/parkour/Blueprint/S_Playerdata` score (`KismetTextLibrary.Conv_StringToText` playerName)))
  (`GameplayStatics.SaveGameToSlot` (`self.recordData`) (`self.slotName`)))