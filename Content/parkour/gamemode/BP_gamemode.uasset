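; Game mode for an endless-runner parkour game that ramps up player speed and recycles track tiles.
; beginggame caches the BP_Land_ actors, PlayerStart and parkour character, then shows the UI_pokerui widget.
; Tick raises the character's walk speed over time up to a cap.
; LoopTrack moves a given tile ahead of the furthest along Y and refreshes its barriers; Addland's spawn logic is disconnected.
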(event `add land`
  (params (landbeging :type "Integer (by ref)") (landend :type "Integer (by ref)"))
  (bind _output_get (set `self.Landend` landend))
  (for _index (range landbeging (+ _output_get 1))
    (`self.addland` _index)))

(event `beging game`
  (bind _outactors (`GameplayStatics.GetAllActorsOfClass` "/Game/parkour/Blueprint/BP_Land_.BP_Land__C"))
  (set `self.landarray` _outactors)
  (bind _returnvalue (`GameplayStatics.GetActorOfClass` "/Script/Engine.PlayerStart"))
  (set `self.PlayerStart` _returnvalue)
  (bind _asbp_parkourchr (cast `/Game/parkour/Blueprint/BP_parkourchr` (`GameplayStatics.GetPlayerPawn` 0)))
  (set `self.As BP Parkourchr` _asbp_parkourchr)
  (bind _returnvalue_2 (`|CreateWidget` "/Game/parkour/UI/UI_pokerui.UI_pokerui_C"))
  (`UserWidget.AddToViewport` _returnvalue_2 0))

(event `self.ReceiveTick`
  (params (DeltaSeconds :type "Float (single-precision)"))
  (bind _as_bp_parkourchr (`self.As BP Parkourchr`))
  (bind _charactermovement (`Character.CharacterMovement` _as_bp_parkourchr))
  ; set actor speed
  (`/Engine/EditorBlueprintResources/StandardMacros.IsValid` _as_bp_parkourchr
    (:`Is Valid`
      (set `CharacterMovementComponent.MaxWalkSpeed` (`KismetMathLibrary.FClamp` (+ (`CharacterMovementComponent.MaxWalkSpeed` _charactermovement) (* (`self.Acceleration`) (`GameplayStatics.GetWorldDeltaSeconds`))) 0.0 1500.0) _charactermovement))))

(fn `addland`
  (params (index :type Integer)))

(fn `LoopTrack`
  (params (land :type "/Game/parkour/Blueprint/BP_Land_ Object Reference"))
  (locals (FrontLand :type "/Game/parkour/Blueprint/BP_Land_ Object Reference") (Maxx :type "Float (double-precision)" :default -1000.0))
  (bind (_returnvalue_x _returnvalue_y _returnvalue_z) (`KismetMathLibrary.BreakVector` (`self.K2_GetActorLocation` (`local.FrontLand`))))
  (for _array_element (`self.landarray`)
    (bind (_returnvalue_x_2 _returnvalue_y_2) (`KismetMathLibrary.BreakVector` (`self.K2_GetActorLocation` _array_element)))
    (if (> _returnvalue_y_2 (`local.Maxx`))
      (set `local.Maxx` _returnvalue_y_2)
      (set `local.FrontLand` _array_element)))
  (`self.K2_SetActorLocation` land (`KismetMathLibrary.MakeVector` _returnvalue_x (+ _returnvalue_y (`self.Tilelength`)) _returnvalue_z) false false)
  (for _array_element_2 (`/Game/parkour/Blueprint/BP_Land_.piece array` land)
    (`/Game/parkour/Blueprint/BP_land_piece.unable all barrier and tool` _array_element_2))
  (`/Game/parkour/Blueprint/BP_Land_.Add barriers` land))

(fn `UserConstructionScript`)